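; Construction site proxy that shows a building's mesh in a ghost material, with entrance and collision box fitted to it, until work finishes.
; Each tick it advances a work clock using the game-speed time unit, kept in sync through GameState, divided by the count of workers who reported to shift.
; Once work time reaches construction time, it signals completion, frees its workers and destroys itself after a short delay.
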(event `self.ReceiveBeginPlay`
  ;[1 0.07939 0] Begin Play
  (bind _output_get (set `self.GameStateRef` (cast `/Game/_Blueprints/GameBPs/MyGameState` (`GameplayStatics.GetGameState`) :!pure true)))
  (add `/Game/_Blueprints/GameBPs/MyGameState.UpdateGameSpeed` _output_get (`|CreateDelegate` :!event `AdjustTime`))
  (bind _timeunit (`/Game/_Blueprints/GameBPs/MyGameState.GetCurrentTimeUnit` (`self.GameStateRef`)))
  (set `self.TimeUnit` _timeunit))

(event `self.ReceiveTick`
  (params (DeltaSeconds :type "Float (single-precision)"))
  ;[0.9652 0.08209 1] Tick
  (set `self.Delta` DeltaSeconds)
  (if (not (`self.IsConstructionCompleted`))
    (`self.DoWork`)
    (if (>= (`self.WorkTimeSpent`) (`self.ConstructionTime`))
      (set `self.IsConstructionCompleted` true)
      (`self.ConstructionCompleted` self)
      (`self.ConstructionIsComplete`)
      (`KismetSystemLibrary.Delay` 0.2)
      (`self.K2_DestroyActor`))))

(event `AdjustTime`
  (params (TimeUnit :type "Float (double-precision)"))
  ;[0.03349 0.5098 1] Adjust Time
  (set `self.TimeUnit` TimeUnit))

(fn `ConstructionIsComplete`
  (if (> (`self.GetWorkforce`) 0.0)
    (for _array_element (`self.ActiveWorkers`)
      (`/Game/_Blueprints/Construction/Workers/Worker_BP.SetIsBusy` _array_element false))
    (set `self.ActiveWorkers` (`|MakeArray` null :!type "/Game/_Blueprints/Construction/Workers/Worker_BP Object Reference"))
    (return)
    (else
      (return))))

(fn `DoWork`
  (bind _active_workers (`self.GetWorkforce`))
  (if (> _active_workers 0.0)
    (bind _output_get (set `self.ClockWork` (`/Game/_Blueprints/Libraries/FunctionLibrary.SetClockWork` (`self.Delta`) (/ (`self.TimeUnit`) _active_workers) (`self.ClockWork`))))
    (set `self.WorkTimeSpent` (* _output_get 60.0))
    (return)
    (else
      (return))))

(fn `GetWorkforce`
  (returns (`Active Workers` :type "Float (double-precision)"))
  (return (`KismetMathLibrary.Conv_IntToDouble` (`KismetArrayLibrary.Array_Length` (`self.ActiveWorkers`)))))

(fn `ReportToShift`
  (params (Worker :type "/Game/_Blueprints/Construction/Workers/Worker_BP Object Reference"))
  (`KismetArrayLibrary.Array_Add` (`self.ActiveWorkers`) Worker)
  (return))

(fn `SetConstructionTime`
  (params (WorkHours :type "Float (double-precision)"))
  (set `self.ConstructionTime` (* WorkHours 60.0))
  (return))

(fn `UserConstructionScript`
  (bind _staticmesh (`self.StaticMesh`))
  (`StaticMeshComponent.SetStaticMesh` _staticmesh (`self.DisplayMesh`))
  (`PrimitiveComponent.SetMaterial` _staticmesh 0 "/Game/_Resources/Rendering/GhostBuildingsMaterialsMaterials/Ghost_M_Inst.Ghost_M_Inst")
  (`/Game/_Blueprints/Libraries/FunctionLibrary.SetBuildingEntrance` (`self.Entrance`) (`self.StaticMesh`))
  (`/Game/_Blueprints/Libraries/FunctionLibrary.SetBuildingCollisionBox` (`self.Collision`) (`self.StaticMesh`)))