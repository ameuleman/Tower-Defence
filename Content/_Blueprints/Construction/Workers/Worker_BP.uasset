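; Worker NPC for the construction system, driven by a Worker AI controller that is cached on BeginPlay.
; The construction script randomizes each worker's sex, tints a dynamic body material to match, and stores a profile with that sex and a random name.
; Names come from random entries in separate male and female name enums.
; SetIsBusy writes the worker's busy state to the controller's Blackboard.
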(event `self.ReceiveBeginPlay`
  (set `self.AIControllerRef` (cast `/Game/_Blueprints/Construction/Workers/Worker_AIController` (`AIBlueprintHelperLibrary.GetAIController` self) :!pure true)))

(fn `GetRandomName`
  (params (Sex :type "/Game/_Blueprints/Enums/NPCSexType_ENUM Enum" :default "NewEnumerator0"))
  (returns (Name :type String))
  (if (`|EnumEquality` Sex "NewEnumerator0")
    (return (`|GetEnumeratorNameAsString` (enumliteral `/Game/_Blueprints/Enums/NPCNameMale_ENUM` (cast `/Game/_Blueprints/Enums/NPCNameMale_ENUM` (`KismetMathLibrary.Conv_IntToByte` (`KismetMathLibrary.RandomIntegerInRange` 0 (- (enumcount `/Game/_Blueprints/Enums/NPCNameMale_ENUM`) 1)))))))
    (else
      (return (`|GetEnumeratorNameAsString` (enumliteral `/Game/_Blueprints/Enums/NPCNameFemale_ENUM` (cast `/Game/_Blueprints/Enums/NPCNameFemale_ENUM` (`KismetMathLibrary.Conv_IntToByte` (`KismetMathLibrary.RandomIntegerInRange` 0 (- (enumcount `/Game/_Blueprints/Enums/NPCNameFemale_ENUM`) 1))))))))))

(fn `RandomNPCFeatures`
  (locals (MaterialInstance :type "MaterialInstanceDynamic Object Reference") (FemaleColor :type "LinearColor Structure" :default (struct :`R` 0.451 :`G` 0.028 :`B` 0.266)) (MaleColor :type "LinearColor Structure" :default (struct :`R` 0.061 :`G` 0.107 :`B` 0.451)))
  (bind _materialinstance (`local.MaterialInstance`))
  (bind _returnvalue (`PrimitiveComponent.CreateDynamicMaterialInstance` (`self.Mesh`) 0 "/Game/_Resources/Rendering/Mannequin/Character/Materials/M_UE4Man_Body_Inst.M_UE4Man_Body_Inst"))
  (set `local.MaterialInstance` _returnvalue)
  (if (`|EnumEquality` (enumliteral `/Game/_Blueprints/Enums/NPCSexType_ENUM` (cast `/Game/_Blueprints/Enums/NPCSexType_ENUM` (`KismetMathLibrary.Conv_IntToByte` (`KismetMathLibrary.RandomIntegerInRange` 0 1)))) "NewEnumerator0")
    (`MaterialInstanceDynamic.SetVectorParameterValue` _materialinstance "BodyColor" (`local.MaleColor`))
    (bind _name (`self.GetRandomName` "NewEnumerator0"))
    (set `self.MyProfile` (make `/Game/_Blueprints/Structs/NPCProfile_Struct` _name))
    (else
      (`MaterialInstanceDynamic.SetVectorParameterValue` _materialinstance "BodyColor" (`local.FemaleColor`))
      (bind _name_2 (`self.GetRandomName` "NewEnumerator1"))
      (set `self.MyProfile` (make `/Game/_Blueprints/Structs/NPCProfile_Struct` _name_2 "NewEnumerator1")))))

(fn `SetIsBusy`
  (params (IsBusy :type Boolean))
  (`BlackboardComponent.SetValueAsBool` (`AIBlueprintHelperLibrary.GetBlackboard` (`self.AIControllerRef`)) (`self.IsBusy`) IsBusy)
  (return))

(fn `UserConstructionScript`
  (`self.RandomNPCFeatures`))