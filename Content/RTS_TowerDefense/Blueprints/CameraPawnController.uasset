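; Player controller for an RTS tower defense game, handling camera, building placement, gatherer purchases and the win/lose screen.
; On BeginPlay it spawns the construction manager, ghost building, HUD and starting workers.
; The cursor-following, rotatable ghost either queues tech buildings with the manager or spawns defenses directly, charging HUD-held resources.
; Camera input drives CameraPawn through zoom-scaled axis movement, screen-edge scrolling, gated mouse rotation and spring-arm zoom.
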(event `self.ReceiveBeginPlay`
  (bind _returnvalue (`KismetMathLibrary.MakeTransform` (0.0 0.0 0.0) (struct) (1.0 1.0 1.0)))
  ;[1 0 0] Begin
  (`|ExecutionSequence`
    (:`then_0`
      (`self.ReferenceCasts`))
    (:`then_1`
      (bind _returnvalue_2 (`|SpawnActorFromClass` "/Game/RTS_TowerDefense/Blueprints/Construction/ConstructionManager_BP.ConstructionManager_BP_C" _returnvalue "AlwaysSpawn" "OverrideRootScale"))
      (set `self.ConstructionManagerRef` _returnvalue_2))
    (:`then_2`
      (bind _returnvalue_3 (`|SpawnActorFromClass` "/Game/RTS_TowerDefense/Blueprints/Buildings/TechnologyBuildings/GhostBuilding_BP.GhostBuilding_BP_C" _returnvalue "AlwaysSpawn" "OverrideRootScale" null self))
      (set `self.GhostBuildingRef` _returnvalue_3))
    (:`then_3`
      (`WidgetBlueprintLibrary.SetInputMode_GameAndUIEx` self null true false)
      (`self.CreateHuds`)
      (`UserWidget.AddToViewport` (`self.MainHudRef`) 0))
    (:`then_4`
      ;[1 1 1] BeginPlayInitialWorkers
      (for _index (range 3)
        (bind _outactors (`GameplayStatics.GetAllActorsOfClass` "/Game/ThirdPersonBP/Blueprints/ResourceBuilding.ResourceBuilding_C"))
        (bind _item (`KismetArrayLibrary.Array_Get` _outactors (* _index 3)))
        (bind _returnvalue_4 (`|SpawnActorFromClass` "/Game/ThirdPersonBP/Blueprints/Gatherer.Gatherer_C" (`SceneComponent.K2_GetComponentToWorld` (`/Game/ThirdPersonBP/Blueprints/ResourceBuilding.Billboard` _item)) "AdjustIfPossibleButAlwaysSpawn" "OverrideRootScale" self _item self))
        (`Pawn.SpawnDefaultController` _returnvalue_4))
      (`|SpawnActorFromClass` "/Game/RTS_TowerDefense/Blueprints/AI/Workers/Worker_BP.Worker_BP_C" (`SceneComponent.K2_GetComponentToWorld` (`/Game/ThirdPersonBP/Blueprints/ResourceBuilding.Billboard` (`KismetArrayLibrary.Array_Get` _outactors 1))) "Undefined" "OverrideRootScale"))))

(event `Key|LeftMouseButton`
  (params (Key :type "Key Structure" :default "AnyKey"))
  (bind _ghostbuildingref (`self.GhostBuildingRef`))
  (bind _mainhudref (`self.MainHudRef`))
  (bind _mainhudref_2 (`self.MainHudRef`))
  (bind (_returnvalue_x _returnvalue_y) (`KismetMathLibrary.BreakVector` (`self.K2_GetActorLocation` _ghostbuildingref)))
  (bind _ressources (`/Game/RTS_TowerDefense/HUDs/MainUI_HUD.Ressources` _mainhudref))
  ;[1 1 1] Left Mouse Button
  (:`Pressed`
    (if (and (`self.BuildModeActive`) (not (`/Game/RTS_TowerDefense/Blueprints/Buildings/TechnologyBuildings/GhostBuilding_BP.GetIsOverlapping` (`self.GhostBuildingRef`))))
      (if (`/Game/RTS_TowerDefense/Blueprints/Buildings/TechnologyBuildings/GhostBuilding_BP.isTechBuilding` _ghostbuildingref)
        (bind _constructionstruct (`/Game/RTS_TowerDefense/Blueprints/Buildings/TechnologyBuildings/GhostBuilding_BP.GetConstructionStruct` (`self.GhostBuildingRef`)))
        (`/Game/RTS_TowerDefense/Blueprints/Construction/ConstructionManager_BP.QueueConstruction` (`self.ConstructionManagerRef`) _constructionstruct)
        (`/Game/RTS_TowerDefense/Blueprints/Buildings/TechnologyBuildings/GhostBuilding_BP.KillGhost` (`self.GhostBuildingRef`))
        (set `/Game/RTS_TowerDefense/HUDs/MainUI_HUD.Ressources` (- (`/Game/RTS_TowerDefense/HUDs/MainUI_HUD.Ressources` _mainhudref_2) (`/Game/RTS_TowerDefense/HUDs/MainUI_HUD.TempRessourcesCost` _mainhudref_2)) _mainhudref_2)
        (else
          (bind _returnvalue (`|SpawnActorFromClass` (`/Game/RTS_TowerDefense/Blueprints/Buildings/TechnologyBuildings/GhostBuilding_BP.defenseClass` _ghostbuildingref) (`KismetMathLibrary.MakeTransform` (`KismetMathLibrary.MakeVector` _returnvalue_x _returnvalue_y 100.0)) "Undefined" "OverrideRootScale"))
          (`/Engine/EditorBlueprintResources/StandardMacros.IsValid` _returnvalue
            (:`Is Valid`
              (bind _cost (`/Game/RTS_TowerDefense/Blueprints/fightingUnit.cost` _returnvalue))
              (if (>= _ressources _cost)
                (set `/Game/RTS_TowerDefense/HUDs/MainUI_HUD.Ressources` (- _ressources _cost) _mainhudref)
                (else
                  (`self.K2_DestroyActor` _returnvalue)
                  (`KismetSystemLibrary.PrintString` "Ressources insuffisantes !"))))))))))

(event `self.ReceiveTick`
  (params (DeltaSeconds :type "Float (single-precision)"))
  ;[0 0.9757 1] Tick
  (if (`self.BuildModeActive`)
    (if (!= (`self.GhostBuildingRef`) null)
      (`/Game/RTS_TowerDefense/Blueprints/Buildings/TechnologyBuildings/GhostBuilding_BP.SetCursorPosition` (`self.GhostBuildingRef`) (`/Game/RTS_TowerDefense/Libraries/FunctionLibrary.SetCursorWorldPosition` self (`self.SetSightDistance`))))))

(event `InputAction|Deselect`
  (params (Key :type "Key Structure" :default "AnyKey"))
  ;[1 0.4191 0] Deselect
  (:`Pressed`
    (if (`self.BuildModeActive`)
      (`/Game/RTS_TowerDefense/Blueprints/Buildings/TechnologyBuildings/GhostBuilding_BP.KillGhost` (`self.GhostBuildingRef`))
      (set `self.BuildModeActive` false))))

(event `InputAction|RotateBuildingRight`
  (params (Key :type "Key Structure" :default "AnyKey"))
  (bind _ghostbuildingref (`self.GhostBuildingRef`))
  ;[1 1 1] Left Mouse Button
  (:`Pressed`
    (if (and (`KismetSystemLibrary.IsValid` _ghostbuildingref) (`self.BuildModeActive`))
      (`self.K2_SetActorRotation` _ghostbuildingref (`KismetMathLibrary.MakeRotator` (.roll (`self.K2_GetActorRotation` _ghostbuildingref)) (.pitch (`self.K2_GetActorRotation` _ghostbuildingref)) (- (.yaw (`self.K2_GetActorRotation` _ghostbuildingref)) (`self.BuildingRotationRate`))) false))))

(event `InputAction|RotateBuildingLeft`
  (params (Key :type "Key Structure" :default "AnyKey"))
  (bind _ghostbuildingref (`self.GhostBuildingRef`))
  ;[1 1 1] Left Mouse Button
  (:`Pressed`
    (if (and (`KismetSystemLibrary.IsValid` _ghostbuildingref) (`self.BuildModeActive`))
      (`self.K2_SetActorRotation` _ghostbuildingref (`KismetMathLibrary.MakeRotator` (.roll (`self.K2_GetActorRotation` _ghostbuildingref)) (.pitch (`self.K2_GetActorRotation` _ghostbuildingref)) (+ (.yaw (`self.K2_GetActorRotation` _ghostbuildingref)) (`self.BuildingRotationRate`))) false))))

(event `InputAxis|MoveForward`
  (params (AxisValue :type "Float (single-precision)"))
  ;[1 1 1] Camera Movement
  ;;[0.8368 1 0.5136] Movement X
  (if (not (`self.DisableCamNav`))
    (`self.K2_SetActorTransform` (`self.CameraPawnRef`) (`self.MovementX` (`self.MovementSpeedCalculation`) (`self.FastMoveMultiplier`) AxisValue (`self.CameraPawnRef`)) false false)))

(event `InputAxis|MoveRight`
  (params (AxisValue :type "Float (single-precision)"))
  ;[1 1 1] Camera Movement
  ;;[0.09453 0.6525 1] Movement Y
  (if (not (`self.DisableCamNav`))
    (`self.K2_SetActorTransform` (`self.CameraPawnRef`) (`KismetMathLibrary.MakeTransform` (`KismetMathLibrary.MakeVector` (.x (.location (`self.MovementY` AxisValue (`self.MovementSpeedCalculation`) (`self.FastMoveMultiplier`) (`self.CameraPawnRef`)))) (.y (.location (`self.MovementY` AxisValue (`self.MovementSpeedCalculation`) (`self.FastMoveMultiplier`) (`self.CameraPawnRef`)))) 100.0) (.rotation (`self.MovementY` AxisValue (`self.MovementSpeedCalculation`) (`self.FastMoveMultiplier`) (`self.CameraPawnRef`))) (.scale (`self.MovementY` AxisValue (`self.MovementSpeedCalculation`) (`self.FastMoveMultiplier`) (`self.CameraPawnRef`)))) false false)))

(event `InputAction|PanReset`
  (params (Key :type "Key Structure" :default "AnyKey"))
  (bind _camerapawnref (`self.CameraPawnRef`))
  ;[1 1 1] Camera Movement
  ;;[1 0.38 0.02316] View Reset
  (:`Pressed`
    (set `SpringArmComponent.TargetArmLength` 1500.0 (`/Game/RTS_TowerDefense/Blueprints/CameraPawn.SpringArm` (`self.CameraPawnRef`)))
    (`self.K2_SetActorRotation` _camerapawnref (`KismetMathLibrary.MakeRotator` (.roll (`self.K2_GetActorRotation` _camerapawnref)) 0.0 0.0) false)))

(event `InputAxisKey|MouseX`
  (params (AxisValue :type "Float (single-precision)"))
  ;[1 1 1] Camera Movement
  ;;[1 0.09279 0.4187] Pan X
  (`/Engine/EditorBlueprintResources/StandardMacros.Gate` true :!label _label
    (:`Exit`
      (`self.K2_SetActorRotation` (`self.CameraPawnRef`) (`KismetMathLibrary.MakeRotator` (.roll (`self.K2_GetActorRotation` (`self.CameraPawnRef`))) (.pitch (`self.K2_GetActorRotation` (`self.CameraPawnRef`))) (+ (.yaw (`self.K2_GetActorRotation` (`self.CameraPawnRef`))) (* (`self.PanSensitivity`) AxisValue))) false))))

(event `InputAction|Pan`
  (params (Key :type "Key Structure" :default "AnyKey"))
  ;[1 1 1] Camera Movement
  ;;[1 0.09279 0.4187] Pan X
  (:`Pressed`
    (set `self.DisableForPan` true)
    (goto _label :!via `Open`))
  (:`Released`
    (set `self.DisableForPan` false)
    (goto _label :!via `Close`)))

(event `InputAction|ZoomIn`
  (params (Key :type "Key Structure" :default "AnyKey"))
  (bind _springarm (`/Game/RTS_TowerDefense/Blueprints/CameraPawn.SpringArm` (`self.CameraPawnRef`)))
  ;[1 1 1] Camera Movement
  ;;[1 0 0] Zoom In/Out
  (:`Pressed`
    (set `SpringArmComponent.TargetArmLength` (`KismetMathLibrary.FClamp` (- (`SpringArmComponent.TargetArmLength` _springarm) (`self.ZoomSensitivity`)) 500.0 (`self.MaxArmDistance`)) _springarm)))

(event `ROS_SpawnGatherer`
  (params (cost :type "Float (double-precision)"))
  (bind _mainhudref (`self.MainHudRef`))
  (bind _mainhudref_2 (`self.MainHudRef`))
  ;[1 1 1] Spawn Worker
  (bind _outactors (`GameplayStatics.GetAllActorsOfClass` "/Game/ThirdPersonBP/Blueprints/ResourceBuilding.ResourceBuilding_C"))
  (bind _item (`KismetArrayLibrary.Array_Get` _outactors (`KismetMathLibrary.RandomInteger` 9)))
  (bind _returnvalue (`|SpawnActorFromClass` "/Game/ThirdPersonBP/Blueprints/Gatherer.Gatherer_C" (`SceneComponent.K2_GetComponentToWorld` (`/Game/ThirdPersonBP/Blueprints/ResourceBuilding.Billboard` _item)) "AdjustIfPossibleButAlwaysSpawn" "OverrideRootScale" self _item self))
  (`/Engine/EditorBlueprintResources/StandardMacros.IsValid` _returnvalue
    (:`Is Valid`
      (set `/Game/RTS_TowerDefense/HUDs/MainUI_HUD.Ressources` (- (`/Game/RTS_TowerDefense/HUDs/MainUI_HUD.Ressources` _mainhudref_2) cost) _mainhudref_2)
      (`/Engine/EditorBlueprintResources/StandardMacros.IncrementInt` (`/Game/RTS_TowerDefense/HUDs/MainUI_HUD.WorkersAlive` _mainhudref_2)
        (:`  `
          (`Pawn.SpawnDefaultController` _returnvalue)
          (`KismetSystemLibrary.Delay` 0.2)
          (`/Engine/EditorBlueprintResources/StandardMacros.IsValid` _returnvalue
            (:`Is Not Valid`
              (set `/Game/RTS_TowerDefense/HUDs/MainUI_HUD.Ressources` (+ (`/Game/RTS_TowerDefense/HUDs/MainUI_HUD.Ressources` (`self.MainHudRef`)) cost) _mainhudref)
              (`/Engine/EditorBlueprintResources/StandardMacros.IncrementInt` (`/Game/RTS_TowerDefense/HUDs/MainUI_HUD.WorkersAlive` _mainhudref)))))))))

(event `InputAxisKey|MouseY`
  (params (AxisValue :type "Float (single-precision)"))
  ;[1 1 1] Camera Movement
  ;;[1 0.9509 0.06679] Pan Y
  (`/Engine/EditorBlueprintResources/StandardMacros.Gate` true :!label _label_2
    (:`Exit`
      (`self.K2_SetActorRotation` (`self.CameraPawnRef`) (`KismetMathLibrary.MakeRotator` (.roll (`self.K2_GetActorRotation` (`self.CameraPawnRef`))) (`KismetMathLibrary.FClamp` (+ (.pitch (`self.K2_GetActorRotation` (`self.CameraPawnRef`))) (* (`self.PanSensitivity`) AxisValue)) -15.0 45.0) (.yaw (`self.K2_GetActorRotation` (`self.CameraPawnRef`)))) false))))

(event `InputAction|ZoomOut`
  (params (Key :type "Key Structure" :default "AnyKey"))
  (bind _springarm (`/Game/RTS_TowerDefense/Blueprints/CameraPawn.SpringArm` (`self.CameraPawnRef`)))
  ;[1 1 1] Camera Movement
  ;;[1 0 0] Zoom In/Out
  (:`Pressed`
    (set `SpringArmComponent.TargetArmLength` (`KismetMathLibrary.FClamp` (+ (`self.ZoomSensitivity`) (`SpringArmComponent.TargetArmLength` _springarm)) 500.0 (`self.MaxArmDistance`)) _springarm)))

(event `InputAction|Pan`
  (params (Key :type "Key Structure" :default "AnyKey"))
  ;[1 1 1] Camera Movement
  ;;[1 0.9509 0.06679] Pan Y
  (:`Pressed`
    (set `self.DisableForPan` true)
    (goto _label_2 :!via `Open`))
  (:`Released`
    (set `self.DisableForPan` false)
    (goto _label_2 :!via `Close`)))

(event `UpdateResources`
  (params (InResources :type "Float (double-precision)"))
  ;[1 1 1] UpdateResources
  (`self.ROC_UpdateResources` InResources))

(event `InputAxisKey|MouseX`
  (params (AxisValue :type "Float (single-precision)"))
  ;[1 1 1] Camera Movement
  ;;[0 1 0] Edge Movement
  (if (not (`self.DisableForPan`))
    (bind (_deltaxspeed _deltayspeed) (`self.ScreenEdgeMovement` :!label _label_3))
    (`self.K2_AddActorLocalOffset` (`self.CameraPawnRef`) (`KismetMathLibrary.MakeVector` _deltaxspeed _deltayspeed) true false)))

(event `ROC_UpdateResources`
  (params (InResources :type "Float (double-precision)"))
  ;[1 1 1] UpdateResources
  (`/Game/RTS_TowerDefense/HUDs/MainUI_HUD.UpdateResources` (`self.MainHudRef`) InResources))

(event `Key|LeftShift`
  (params (Key :type "Key Structure" :default "AnyKey"))
  (bind _fastmovemultiplier (`self.FastMoveMultiplier`))
  ;[1 1 1] Camera Movement
  ;;[0 0.1691 1] Move Multiplier
  (:`Pressed`
    (set `self.FastMoveMultiplier` (* _fastmovemultiplier 2.0)))
  (:`Released`
    (set `self.FastMoveMultiplier` (/ _fastmovemultiplier 2.0))))

(event `Key|V`
  (params (Key :type "Key Structure" :default "AnyKey")))

(event `InputAxisKey|MouseY`
  (params (AxisValue :type "Float (single-precision)"))
  ;[1 1 1] Camera Movement
  ;;[0 1 0] Edge Movement
  (if (not (`self.DisableForPan`))
    (goto _label_3 :!via `MouseY`)))

(event `endGameEvent`
  (params (won :type Boolean))
  (bind _returnvalue (`GameplayStatics.GetPlayerController` 0))
  ;[1 1 1] endGame
  (`KismetSystemLibrary.Delay` 3.0)
  (bind _returnvalue_2 (`|CreateWidget` "/Game/RTS_TowerDefense/HUDs/FinHUD.FinHUD_C" _returnvalue))
  (`UserWidget.AddToViewport` _returnvalue_2 0)
  (if won
    (`Widget.SetVisibility` (`/Game/RTS_TowerDefense/HUDs/FinHUD.img_victoire` _returnvalue_2) "Visible")
    (`GameplayStatics.PlaySound2D` "/Game/RTS_TowerDefense/Sounds/yeha.yeha")
    (else
      (`Widget.SetVisibility` (`/Game/RTS_TowerDefense/HUDs/FinHUD.img_GameOver` _returnvalue_2) "Visible")
      (`GameplayStatics.PlaySound2D` "/Game/RTS_TowerDefense/Sounds/scream.scream")))
  (`GameplayStatics.SetGamePaused` true)
  (set `PlayerController.bShowMouseCursor` true _returnvalue))

(fn `MovementSpeedCalculation`
  (returns (MoveSensitivity :type "Float (double-precision)"))
  (return (`KismetMathLibrary.FClamp` (/ (`SpringArmComponent.TargetArmLength` (`/Game/RTS_TowerDefense/Blueprints/CameraPawn.SpringArm` (`self.CameraPawnRef`))) 100.0) 5.0 20.0)))

(fn `SetCalendar`
  (params (Date :type "Array of Integer (by ref)"))
  (returns (Success :type Boolean))
  (return false))

(fn `SetClock`
  (params (Time :type "Array of Integer (by ref)"))
  (returns (Success :type Boolean))
  (return false))

(fn `SetSightDistance`
  (returns (SightDistance :type "Float (double-precision)"))
  (return (+ (`self.SightDistance`) (`SpringArmComponent.TargetArmLength` (`/Game/RTS_TowerDefense/Blueprints/CameraPawn.SpringArm` (`self.CameraPawnRef`))))))

(fn `UserConstructionScript`)