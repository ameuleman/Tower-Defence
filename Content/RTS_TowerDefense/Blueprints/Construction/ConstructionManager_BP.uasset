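; Construction manager Blueprint that turns queued build orders into finished buildings in the RTS tower defense game.
; Queuing spawns a proxy actor with the display mesh and required work hours, then stores it and its config in parallel Proxies and Queue arrays.
; When a proxy signals completion, its index retrieves the config, the real building replaces it at the same transform, and the main HUD is notified.
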(event `BindConstructionComplete`
  (params (Proxy :type "/Game/RTS_TowerDefense/Blueprints/Construction/ConstructionProxy_BP Object Reference"))
  (add `/Game/RTS_TowerDefense/Blueprints/Construction/ConstructionProxy_BP.ConstructionCompleted` Proxy (`|CreateDelegate` :!event `ConstructionCompleted`)))

(event `ConstructionCompleted`
  (params (Proxy :type "/Game/RTS_TowerDefense/Blueprints/Construction/ConstructionProxy_BP Object Reference"))
  (`self.FinishConstruction` Proxy))

(fn `FinishConstruction`
  (params (Proxy :type "/Game/RTS_TowerDefense/Blueprints/Construction/ConstructionProxy_BP Object Reference"))
  (locals (Index :type Integer :default 0) (Config :type "/Game/RTS_TowerDefense/Structs/ConstructionStruct Structure"))
  (bind _index (`local.Index`))
  (bind _proxies (`self.Proxies`))
  (bind _queue (`self.Queue`))
  (bind (_buildingclass _proxyclass _transform) (break `/Game/RTS_TowerDefense/Structs/ConstructionStruct` (`local.Config`)))
  (bind _output_get (set `local.Index` (`KismetArrayLibrary.Array_Find` _proxies Proxy)))
  (set `local.Config` (`|GetArrayItem` _queue _output_get))
  (`KismetArrayLibrary.Array_Remove` _queue _index)
  (`KismetArrayLibrary.Array_Remove` _proxies _index)
  (`|SpawnActorFromClass` _buildingclass _transform "AlwaysSpawn" "OverrideRootScale" null null null)
  (`self.K2_DestroyActor` Proxy)
  (bind _ascamera_pawn_controller (cast `/Game/RTS_TowerDefense/Blueprints/CameraPawnController` (`GameplayStatics.GetPlayerController` 0)))
  (`/Game/_HUDs/MainUI_HUD.IsBuilded` (`/Game/RTS_TowerDefense/Blueprints/CameraPawnController.MainHudRef` _ascamera_pawn_controller) _buildingclass))

(fn `QueueConstruction`
  (params (ConstructionStruct :type "/Game/RTS_TowerDefense/Structs/ConstructionStruct Structure"))
  (bind (_buildingclass _proxyclass _transform _displaymesh _workhoursrequired) (break `/Game/RTS_TowerDefense/Structs/ConstructionStruct` ConstructionStruct))
  (bind _returnvalue (`|SpawnActorFromClass` _proxyclass _transform "AlwaysSpawn" "OverrideRootScale" null _displaymesh null))
  (`self.BindConstructionComplete` _returnvalue)
  (`KismetArrayLibrary.Array_Add` (`self.Proxies`) _returnvalue)
  (`KismetArrayLibrary.Array_Add` (`self.Queue`) ConstructionStruct)
  (`/Game/RTS_TowerDefense/Blueprints/Construction/ConstructionProxy_BP.SetConstructionTime` _returnvalue _workhoursrequired))

(fn `UserConstructionScript`)