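; Placement ghost for tech and defense buildings in build mode, previewing where a building can go.
; It spawns and immediately destroys an instance of the chosen class to copy its mesh and build data.
; A gated Tick grid-snaps to the cursor position, then checks BuildingArea overlap and uses corner and center traces to test slope and settle height.
; Invalid spots switch to an error material, and GetConstructionStruct packages the construction data.
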(event `OnSpawn`
  (params (buildingArea :type "Actor Class Reference") (displaySkeletalMesh :type "SkeletalMesh Object Reference") (capsule :type "CapsuleComponent Object Reference") (fightingBuildingClass :type "/Game/RTS_TowerDefense/Blueprints/Buildings/FightingBuildings/DefendedInstallation Class Reference") (DisplayStaticMesh :type "StaticMesh Object Reference") (BuildingClass :type "/Game/RTS_TowerDefense/Blueprints/Buildings/TechnologyBuildings/BuildingMaster_BP Class Reference") (ConstructionProxy :type "/Game/RTS_TowerDefense/Blueprints/Construction/ConstructionProxy_BP Class Reference") (WorkHours :type "Float (double-precision)"))
  (bind _arrow (`self.Arrow`))
  (bind _returnvalue (not (`self.IsOverlapping`)))
  ;[0.02832 1 0] On Spawn Ghost
  (if (not (`self.IsActive`))
    (set `self.buildingArea` buildingArea)
    (set `self.displaySkeletalMesh` displaySkeletalMesh)
    (set `self.capsuleRef` capsule)
    (set `self.defenseClass` fightingBuildingClass)
    (set `self.DisplayStaticMesh` DisplayStaticMesh)
    (set `self.BuildingClass` BuildingClass)
    (set `self.ConstructionProxy` ConstructionProxy)
    (set `self.WorkHoursRequired` WorkHours)
    (set `self.IsActive` true)
    (set `/Game/RTS_TowerDefense/Blueprints/CameraPawnController.BuildModeActive` true (`self.ControllerRef`))
    (if (`self.isTechBuilding`)
      (`StaticMeshComponent.SetStaticMesh` (`self.GhostBuilding_Mesh`) (`self.DisplayStaticMesh`))
      (`self.OpenTickGate`)
      (`self.SetMaterialFun` _returnvalue)
      (bind _output_get (set `self.Extent` (`.BoxExtent` (`KismetSystemLibrary.GetComponentBounds` (`self.GhostBuilding_Mesh`)))))
      (`SceneComponent.K2_SetRelativeLocation` _arrow (`KismetMathLibrary.MakeVector` 0.0 (.y _output_get)) false false)
      (`SceneComponent.SetHiddenInGame` _arrow false false)
      (`/Game/RTS_TowerDefense/Libraries/FunctionLibrary.SetBuildingCollisionBox` (`self.Collision`) (`self.GhostBuilding_Mesh`))
      (`SceneComponent.SetVisibility` (`self.Collision`) true false)
      (else
        (`SkinnedMeshComponent.SetSkinnedAssetAndUpdate` (`self.defenseBuildingMesh`) (`self.displaySkeletalMesh`) true)
        (`self.OpenTickGate`)
        (`self.SetMaterialFun` _returnvalue)
        (set `self.Extent` (`.BoxExtent` (`KismetSystemLibrary.GetComponentBounds` (`self.GhostBuilding_Mesh`))))
        (bind _output_get_2 (set `self.Capsule` (`self.capsuleRef`)))
        (`PrimitiveComponent.SetCollisionResponseToAllChannels` _output_get_2 "ECR_Overlap")))))

(event `KillGhost`
  ;[1 0.0578 0] Kill Ghost
  (set `self.buildingArea` null)
  (set `self.defenseClass` null)
  (set `self.BuildingClass` null)
  (set `self.ConstructionProxy` null)
  (`self.CloseTickGate`)
  (set `self.displaySkeletalMesh` null)
  (set `self.DisplayStaticMesh` null)
  (set `self.IsActive` false)
  (set `/Game/RTS_TowerDefense/Blueprints/CameraPawnController.BuildModeActive` false (`self.ControllerRef`))
  (`SkinnedMeshComponent.SetSkinnedAssetAndUpdate` (`self.defenseBuildingMesh`) (`self.displaySkeletalMesh`) true)
  (`StaticMeshComponent.SetStaticMesh` (`self.GhostBuilding_Mesh`) (`self.DisplayStaticMesh`))
  (`self.K2_SetActorRotation` (struct))
  (`SceneComponent.SetHiddenInGame` (`self.Arrow`) true false)
  (set `self.Extent` (0.0 0.0 0.0))
  (set `self.Capsule` null)
  (`BoxComponent.SetBoxExtent` (`self.Collision`) (0.0 0.0 0.0) false))

(event `/Game/RTS_TowerDefense/Interfaces/I_HUD.ConstructBuilding`
  (params (MainBuilding :type "/Game/RTS_TowerDefense/Blueprints/Buildings/TechnologyBuildings/BuildingMaster_BP Class Reference"))
  ;[0.003043 0.5675 1] Construct Building
  (set `self.isTechBuilding` true)
  (bind _returnvalue (`|SpawnActorFromClass` MainBuilding (`KismetMathLibrary.MakeTransform` (0.0 0.0 0.0)) "Undefined" "OverrideRootScale" null (`self.ControllerRef`)))
  (`|ExecutionSequence`
    (:`then_0`
      (bind _asbuilding_master_bp (castclass `/Game/RTS_TowerDefense/Blueprints/Buildings/TechnologyBuildings/BuildingMaster_BP` MainBuilding))
      (`self.KillGhost`)
      (`self.OnSpawn` (`/Game/RTS_TowerDefense/Blueprints/Buildings/TechnologyBuildings/BuildingMaster_BP.buildingArea` _returnvalue) null null null (`/Game/RTS_TowerDefense/Blueprints/Buildings/TechnologyBuildings/BuildingMaster_BP.DisplayMesh` _returnvalue) _asbuilding_master_bp (`/Game/RTS_TowerDefense/Blueprints/Buildings/TechnologyBuildings/BuildingMaster_BP.ConstructionProxy` _returnvalue) (`/Game/RTS_TowerDefense/Blueprints/Buildings/TechnologyBuildings/BuildingMaster_BP.ConstructionTime` _returnvalue)))
    (:`then_1`
      (`self.K2_DestroyActor` _returnvalue))))

(event `/Game/RTS_TowerDefense/Interfaces/I_HUD.placeDefense`
  (params (defenseClass :type "/Game/RTS_TowerDefense/Blueprints/Buildings/FightingBuildings/DefendedInstallation Class Reference"))
  ;[0.003043 0.5675 1] Place defense
  (set `self.isTechBuilding` false)
  (bind _returnvalue (`|SpawnActorFromClass` defenseClass (`KismetMathLibrary.MakeTransform` (0.0 0.0 0.0) (struct) (1.0 1.0 1.0)) "Undefined" "OverrideRootScale"))
  (`|ExecutionSequence`
    (:`then_0`
      (`self.KillGhost`)
      (`self.OnSpawn` (`/Game/RTS_TowerDefense/Blueprints/Buildings/FightingBuildings/DefendedInstallation.buildingArea` _returnvalue) (`SkinnedMeshComponent.SkeletalMesh` (`Character.Mesh` _returnvalue)) (`Character.CapsuleComponent` _returnvalue) defenseClass))
    (:`then_1`
      (`self.K2_DestroyActor` _returnvalue))))

(event `self.ReceiveTick`
  (params (DeltaSeconds :type "Float (single-precision)"))
  (bind (_gridsnap_x _gridsnap_y) (`KismetMathLibrary.BreakVector` (`self.SetGridSnapVector`)))
  ;[0.295 0.2494 0.00463] Tick
  (`/Engine/EditorBlueprintResources/StandardMacros.Gate` true :!label _label
    (:`Exit`
      (`self.K2_SetActorLocation` self (`KismetMathLibrary.MakeVector` _gridsnap_x _gridsnap_y) false false)
      (if (`self.CheckOverlap`)
        (`self.SetMaterialFun` true)
        (else
          (bind _badlocation (`self.CalculateSlope`))
          (`self.SetMaterialFun` _badlocation))))))

(event `OpenTickGate`
  ;[0.295 0.2494 0.00463] Tick
  (goto _label :!via `Open`))

(event `CloseTickGate`
  ;[0.295 0.2494 0.00463] Tick
  (goto _label :!via `Close`))

(event `SetMaterialFun`
  (params (IsError :type Boolean))
  (bind _defensebuildingmesh (`self.defenseBuildingMesh`))
  ;[1 0 0.9989] Set Material
  (if (not (== IsError (`self.IsOverlapping`)))
    (set `self.IsOverlapping` IsError)
    (if (`self.IsOverlapping`)
      (set `self.currentMaterial` "/Game/RTS_TowerDefense/Materials/GhostError_M_Inst.GhostError_M_Inst")
      (else
        (set `self.currentMaterial` "/Game/RTS_TowerDefense/Materials/Ghost_M_Inst.Ghost_M_Inst")))
    (if (`self.isTechBuilding`)
      (`PrimitiveComponent.SetMaterial` (`self.GhostBuilding_Mesh`) 0 (`self.currentMaterial`))
      (else
        (for (_ _array_index) (`MeshComponent.GetMaterials` _defensebuildingmesh)
          (`PrimitiveComponent.SetMaterial` _defensebuildingmesh _array_index (`self.currentMaterial`)))))))

(fn `CalculateSlope`
  (returns (BadLocation :type Boolean))
  (locals (Differences :type "Array of Float (double-precision)") (MaxDifferences :type "Float (double-precision)" :default 20.0))
  (bind (_actorlocation _forwardvector _rightvector) (`self.GetVectors`))
  (bind (_actorlocation_2 _forwardvector_2 _rightvector_2) (`self.GetVectors`))
  (bind (_actorlocation_3 _forwardvector_3 _rightvector_3) (`self.GetVectors`))
  (bind (_actorlocation_4 _forwardvector_4 _rightvector_4) (`self.GetVectors`))
  (bind _actorlocation_5 (`self.GetVectors`))
  (bind _actorlocation_6 (`self.GetVectors`))
  (bind _differences (`local.Differences`))
  (bind (_extent_x _extent_y) (`KismetMathLibrary.BreakVector` (`self.Extent`)))
  (bind _maxdifferences (`local.MaxDifferences`))
  (bind (_indexofminvalue _minvalue) (`KismetMathLibrary.MinOfFloatArray` _differences))
  (bind (_indexofmaxvalue _maxvalue) (`KismetMathLibrary.MaxOfFloatArray` _differences))
  (`|ExecutionSequence`
    (:`then_0`
      (`|ExecutionSequence`
        (:`then_0`
          (bind _difference (`self.SlopeTrace` (+ _actorlocation (* (+ _forwardvector _rightvector) (`self.Extent`)))))
          (`KismetArrayLibrary.Array_Add` (`local.Differences`) _difference))
        (:`then_1`
          (bind _difference_2 (`self.SlopeTrace` (+ _actorlocation_2 (* (+ (* _forwardvector_2 -1.0) _rightvector_2) (`self.Extent`)))))
          (`KismetArrayLibrary.Array_Add` (`local.Differences`) _difference_2))
        (:`then_2`
          (bind _difference_3 (`self.SlopeTrace` (+ _actorlocation_3 (* (+ _forwardvector_3 (* _rightvector_3 -1.0)) (`self.Extent`)))))
          (`KismetArrayLibrary.Array_Add` (`local.Differences`) _difference_3))
        (:`then_3`
          (bind _difference_4 (`self.SlopeTrace` (+ _actorlocation_4 (* (+ (* _forwardvector_4 -1.0) (* _rightvector_4 -1.0)) (`self.Extent`)))))
          (`KismetArrayLibrary.Array_Add` (`local.Differences`) _difference_4))
        (:`then_4`
          (bind _difference_5 (`self.SlopeTrace` (`self.GetVectors`)))
          (`KismetArrayLibrary.Array_Add` (`local.Differences`) _difference_5))))
    (:`then_1`
      (if (and (> _indexofminvalue -1) (> _indexofmaxvalue -1))
        (bind (_outhit _returnvalue) (`KismetSystemLibrary.BoxTraceSingle` (+ _actorlocation_5 (0.0 0.0 1000.0)) (- _actorlocation_5 (0.0 0.0 1000.0)) (`KismetMathLibrary.MakeVector` _extent_x _extent_y 1.0) (struct) "TraceTypeQuery3"))
        (if _returnvalue
          (`self.K2_SetActorLocation` (`KismetMathLibrary.MakeVector` (.x _actorlocation_6) (.y _actorlocation_6) (.z (`.ImpactPoint` (`GameplayStatics.BreakHitResult` _outhit))))))))
    (:`then_2`
      (return (or (> (`KismetMathLibrary.Abs` _minvalue) _maxdifferences) (> (`KismetMathLibrary.Abs` _maxvalue) _maxdifferences))))))

(fn `CheckOverlap`
  (returns (Overlapping :type Boolean))
  (bind _returnvalue (`KismetArrayLibrary.Array_Length` (`self.GetOverlappingActors` (`self.buildingArea`))))
  (return (or (> (`KismetArrayLibrary.Array_Length` (`self.GetOverlappingActors` "/Script/Engine.Actor")) _returnvalue) (<= _returnvalue 0))))

(fn `GetConstructionStruct`
  (returns (ConstructionStruct :type "/Game/RTS_TowerDefense/Structs/ConstructionStruct Structure"))
  (bind (_returnvalue_x _returnvalue_y) (`KismetMathLibrary.BreakVector` (`self.K2_GetActorLocation`)))
  (return (make `/Game/RTS_TowerDefense/Structs/ConstructionStruct` (`self.BuildingClass`) (`self.ConstructionProxy`) (`KismetMathLibrary.MakeTransform` (`KismetMathLibrary.MakeVector` _returnvalue_x _returnvalue_y) (`self.K2_GetActorRotation`) (1.0 1.0 1.0)) (`self.DisplayStaticMesh`) (`self.WorkHoursRequired`))))

(fn `GetIsOverlapping`
  (returns (IsOverlapping :type Boolean))
  (return (`self.IsOverlapping`)))

(fn `GetVectors`
  (returns (ActorLocation :type "Vector Structure") (ForwardVector :type "Vector Structure") (RightVector :type "Vector Structure"))
  (bind _returnvalue (`self.K2_GetActorRotation`))
  (return (`self.K2_GetActorLocation`) (`KismetMathLibrary.GetForwardVector` _returnvalue) (`KismetMathLibrary.GetRightVector` _returnvalue)))

(fn `SetCalendar`
  (params (Date :type "Array of Integer (by ref)"))
  (returns (Success :type Boolean))
  (return false))

(fn `SetClock`
  (params (Time :type "Array of Integer (by ref)"))
  (returns (Success :type Boolean))
  (return false))

(fn `SetCursorPosition`
  (params (CursorLocation :type "Vector Structure"))
  (set `self.CursorWorldPosition` CursorLocation)
  (return))

(fn `SetGridSnapVector`
  (returns (GridSnap :type "Vector Structure"))
  (bind (_cursorworldposition_x _cursorworldposition_y _cursorworldposition_z) (`KismetMathLibrary.BreakVector` (`self.CursorWorldPosition`)))
  (bind _gridsize (`self.GridSize`))
  (return (`KismetMathLibrary.MakeVector` (`/Game/RTS_TowerDefense/Libraries/FunctionLibrary.GridSnap` _cursorworldposition_x _gridsize) (`/Game/RTS_TowerDefense/Libraries/FunctionLibrary.GridSnap` _cursorworldposition_y _gridsize) (`/Game/RTS_TowerDefense/Libraries/FunctionLibrary.GridSnap` _cursorworldposition_z _gridsize))))

(fn `SlopeTrace`
  (params (TraceLocation :type "Vector Structure"))
  (returns (Difference :type "Float (double-precision)"))
  (bind (_returnvalue_x _returnvalue_y _returnvalue_z) (`KismetMathLibrary.BreakVector` (`self.K2_GetActorLocation`)))
  (bind _outhit (`KismetSystemLibrary.LineTraceSingle` (+ TraceLocation (0.0 0.0 1000.0)) (- TraceLocation (0.0 0.0 1000.0)) "TraceTypeQuery3"))
  (return (- _returnvalue_z (.z (`.ImpactPoint` (`GameplayStatics.BreakHitResult` _outhit))))))

(fn `UserConstructionScript`)