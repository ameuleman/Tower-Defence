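; Resource deposit for the RTS tower defense worker economy that fills its site box with resource actors and regrows them over time.
; On BeginPlay it recursively spawns resources at random points and yaws, retrying failed spawns, until start capacity is reached.
; A looping timer then attempts one spawn per tick while below max capacity.
; Each resource references its deposit and carries a full or remainder amount, added to current capacity.
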(event `ROS_SpawnDefaultResource`
  (`self.SpawnDefaultResource`))

(event `self.ReceiveBeginPlay`
  (`self.ROS_SpawnDefaultResource`)
  (`KismetSystemLibrary.K2_SetTimer` null "ROS_Regenerate" 3.0 true))

(event `ROS_Regenerate`
  (`self.Regenerate`))

(fn `Regenerate`
  (bind (_returnvalue_x _returnvalue_y _returnvalue_z) (`KismetMathLibrary.BreakVector` (`self.K2_GetActorLocation`)))
  (bind _depositmaxcapacity (`self.DepositMaxCapacity`))
  (bind _depositsitebox (`self.DepositSiteBox`))
  (if (!= (`self.DepositCurrentCapacity`) (`self.DepositMaxCapacity`))
    (bind _returnvalue (`|SpawnActorFromClass` (`self.ResourceClass`) (`KismetMathLibrary.MakeTransform` (`KismetMathLibrary.MakeVector` (.x (`KismetMathLibrary.RandomPointInBoundingBox` (`SceneComponent.K2_GetComponentLocation` _depositsitebox) (`BoxComponent.GetScaledBoxExtent` _depositsitebox))) (.y (`KismetMathLibrary.RandomPointInBoundingBox` (`SceneComponent.K2_GetComponentLocation` _depositsitebox) (`BoxComponent.GetScaledBoxExtent` _depositsitebox))) _returnvalue_z) (`KismetMathLibrary.MakeRotator` 0.0 0.0 (`KismetMathLibrary.Conv_IntToDouble` (`KismetMathLibrary.RandomIntegerInRange` -180 180)))) "AdjustIfPossibleButDontSpawnIfColliding" "OverrideRootScale" null self))
    (`/Engine/EditorBlueprintResources/StandardMacros.IsValid` _returnvalue
      (:`Is Valid`
        (bind _maxresourcecarry (`/Game/ThirdPersonBP/Blueprints/MasterResource.MaxResourceCarry` _returnvalue))
        (bind _returnvalue_2 (+ (`self.DepositCurrentCapacity`) _maxresourcecarry))
        (if (> _depositmaxcapacity _returnvalue_2)
          (`KismetSystemLibrary.PrintString` (`KismetStringLibrary.Conv_DoubleToString` _maxresourcecarry))
          (bind _output_get (set `/Game/ThirdPersonBP/Blueprints/MasterResource.CurrentResourceCarry` _maxresourcecarry _returnvalue))
          (set `self.DepositCurrentCapacity` (`KismetMathLibrary.FClamp` (+ (`self.DepositCurrentCapacity`) _output_get) 0.0 (`self.DepositMaxCapacity`)))
          (else
            (bind _returnvalue_3 (- _maxresourcecarry (- _returnvalue_2 _depositmaxcapacity)))
            (`KismetSystemLibrary.PrintString` (`KismetStringLibrary.Conv_DoubleToString` _returnvalue_3))
            (bind _output_get_2 (set `/Game/ThirdPersonBP/Blueprints/MasterResource.CurrentResourceCarry` _returnvalue_3 _returnvalue))
            (set `self.DepositCurrentCapacity` (`KismetMathLibrary.FClamp` (+ (`self.DepositCurrentCapacity`) _output_get_2) 0.0 (`self.DepositMaxCapacity`)))))
        (`KismetArrayLibrary.Array_Add` (`self.ResourceInDeposit`) _returnvalue)))))

(fn `SpawnDefaultResource`
  (bind (_returnvalue_x _returnvalue_y _returnvalue_z) (`KismetMathLibrary.BreakVector` (`self.K2_GetActorLocation`)))
  (bind _depositstartcapacity (`self.DepositStartCapacity`))
  (bind _depositsitebox (`self.DepositSiteBox`))
  (bind _returnvalue (`|SpawnActorFromClass` (`self.ResourceClass`) (`KismetMathLibrary.MakeTransform` (`KismetMathLibrary.MakeVector` (.x (`KismetMathLibrary.RandomPointInBoundingBox` (`SceneComponent.K2_GetComponentLocation` _depositsitebox) (`BoxComponent.GetScaledBoxExtent` _depositsitebox))) (.y (`KismetMathLibrary.RandomPointInBoundingBox` (`SceneComponent.K2_GetComponentLocation` _depositsitebox) (`BoxComponent.GetScaledBoxExtent` _depositsitebox))) _returnvalue_z) (`KismetMathLibrary.MakeRotator` 0.0 0.0 (`KismetMathLibrary.Conv_IntToDouble` (`KismetMathLibrary.RandomIntegerInRange` -180 180)))) "AdjustIfPossibleButDontSpawnIfColliding" "OverrideRootScale" null self))
  (`/Engine/EditorBlueprintResources/StandardMacros.IsValid` _returnvalue
    (:`Is Valid`
      (bind _maxresourcecarry (`/Game/ThirdPersonBP/Blueprints/MasterResource.MaxResourceCarry` _returnvalue))
      (bind _returnvalue_2 (+ (`self.DepositCurrentCapacity`) _maxresourcecarry))
      (if (> _depositstartcapacity _returnvalue_2)
        (bind _output_get (set `/Game/ThirdPersonBP/Blueprints/MasterResource.CurrentResourceCarry` _maxresourcecarry _returnvalue))
        (set `self.DepositCurrentCapacity` (+ (`self.DepositCurrentCapacity`) _output_get))
        (`self.SpawnDefaultResource`)
        (else
          (bind _output_get_2 (set `/Game/ThirdPersonBP/Blueprints/MasterResource.CurrentResourceCarry` (- _maxresourcecarry (- _returnvalue_2 _depositstartcapacity)) _returnvalue))
          (set `self.DepositCurrentCapacity` (+ (`self.DepositCurrentCapacity`) _output_get_2))))
      (`KismetArrayLibrary.Array_Add` (`self.ResourceInDeposit`) _returnvalue))
    (:`Is Not Valid`
      (`self.SpawnDefaultResource`))))

(fn `UserConstructionScript`)