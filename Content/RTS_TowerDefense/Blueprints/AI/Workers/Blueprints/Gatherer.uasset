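; Worker unit for the RTS tower-defense game that gathers resources from deposits and delivers them to the player's RTS camera stockpile.
; On startup it picks the nearest non-empty food bush deposit and its nearest resource, then writes targets and state flags to the blackboard.
; Looping timers drive extraction and a multicast-mirrored montage, draining resource and deposit until the bag fills.
; Emptied resources are destroyed and trigger a new search.
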(event `ROS_StartUp`
  (`KismetSystemLibrary.Delay` 0.01)
  (`self.FindDeposit` "NewEnumerator0"))

(event `MC_SetColor`
  (params (Selection :type Name))
  (switch `name` Selection
    (:`TeamOne`
      (`PrimitiveComponent.SetMaterial` (`self.Mesh`) 0 "/Game/ThirdPersonBP/Blueprints/TeamOneMat.TeamOneMat"))
    (:`TeamTwo`
      (`PrimitiveComponent.SetMaterial` (`self.Mesh`) 0 "/Game/ThirdPersonBP/Blueprints/TeamTwoMat.TeamTwoMat"))))

(event `self.ReceiveBeginPlay`
  (`self.ROS_StartUp`))

(event `MC_PlayMontage`
  (`AnimInstance.Montage_Play` (`SkeletalMeshComponent.GetAnimInstance` (`self.Mesh`)) "/Game/ThirdPersonBP/Blueprints/GatheringMontage.GatheringMontage" 1.0 "MontageLength" 0.0))

(event `MC_StopMontage`
  (`AnimInstance.Montage_Stop` (`SkeletalMeshComponent.GetAnimInstance` (`self.Mesh`)) 0.0 "/Game/ThirdPersonBP/Blueprints/GatheringMontage.GatheringMontage"))

(fn `DropOffResource`
  (`/Game/ThirdPersonBP/Blueprints/RTSCam.UpdateResource` (`self.RTSCam`) (`self.CurrentFoodCarry`))
  (set `self.CurrentResourceCarry` 0.0)
  (set `self.CurrentFoodCarry` 0.0)
  (`/Engine/EditorBlueprintResources/StandardMacros.IsValid` (`AIBlueprintHelperLibrary.GetBlackboard` null)
    (:`Is Valid`
      (`BlackboardComponent.SetValueAsBool` (`AIBlueprintHelperLibrary.GetBlackboard` null) (`self.BagFullBBK`) false)
      (`BlackboardComponent.SetValueAsBool` (`AIBlueprintHelperLibrary.GetBlackboard` null) (`self.GoingToResourceBBK`) false)
      (`BlackboardComponent.SetValueAsBool` (`AIBlueprintHelperLibrary.GetBlackboard` null) (`self.ReturningToDropBBK`) false))))

(fn `FindDeposit`
  (params (InDepositType :type "/Game/ThirdPersonBP/Blueprints/ResourceEnum Enum"))
  (locals (LocalDepositElement :type "/Game/ThirdPersonBP/Blueprints/MasterDeposit Object Reference") (LocalValidDeposits :type "Array of /Game/ThirdPersonBP/Blueprints/MasterDeposit Object Reference") (LocalDepositType :type "/Game/ThirdPersonBP/Blueprints/ResourceEnum Enum") (LocalDistanceToDeposit :type "Float (double-precision)"))
  (set `local.LocalDepositType` InDepositType)
  (bind _outactors (`GameplayStatics.GetAllActorsOfClass` "/Game/ThirdPersonBP/Blueprints/MasterDeposit.MasterDeposit_C"))
  (for _array_element _outactors
    (set `local.LocalDepositElement` _array_element)
    (if (and (> (`/Game/ThirdPersonBP/Blueprints/MasterDeposit.DepositCurrentCapacity` (`local.LocalDepositElement`)) 0.0) (`|EnumEquality` (`/Game/ThirdPersonBP/Blueprints/MasterDeposit.DepositType` (`local.LocalDepositElement`)) (`local.LocalDepositType`)))
      (`KismetArrayLibrary.Array_Add` (`local.LocalValidDeposits`) (`local.LocalDepositElement`))))
  (if (> (`KismetArrayLibrary.Array_Length` (`local.LocalValidDeposits`)) 0)
    (for (_array_element_2 _array_index) (`local.LocalValidDeposits`)
      (set `local.LocalDepositElement` _array_element_2)
      (if (== _array_index 0)
        (set `self.CurrentDeposit` (`local.LocalDepositElement`) :!label _label)
        (set `local.LocalDistanceToDeposit` (`self.GetDistanceTo` (`local.LocalDepositElement`) self))
        (elif (< (`self.GetDistanceTo` (`local.LocalDepositElement`) self) (`local.LocalDistanceToDeposit`))
          (goto _label))))
    (`self.FindNearResourceInDeposit`)))

(fn `FindNearResourceInDeposit`
  (locals (LocalResourceInDeposit :type "Array of /Game/ThirdPersonBP/Blueprints/MasterResource Object Reference") (LocalResourceElement :type "/Game/ThirdPersonBP/Blueprints/MasterResource Object Reference") (LocalDistanceToResource :type "Float (double-precision)"))
  (if (> (`/Game/ThirdPersonBP/Blueprints/MasterDeposit.DepositCurrentCapacity` (`self.CurrentDeposit`)) 0.0)
    (bind _output_get (set `local.LocalResourceInDeposit` (`/Game/ThirdPersonBP/Blueprints/MasterDeposit.ResourceInDeposit` (`self.CurrentDeposit`))))
    (for (_array_element _array_index) _output_get
      (set `local.LocalResourceElement` _array_element)
      (if (== _array_index 0)
        (set `self.CurrentResourceToGather` (`local.LocalResourceElement`) :!label _label)
        (set `local.LocalDistanceToResource` (`self.GetDistanceTo` (`local.LocalResourceElement`) self))
        (elif (< (`self.GetDistanceTo` (`local.LocalResourceElement`) self) (`local.LocalDistanceToResource`))
          (goto _label))))
    (`AnimInstance.Montage_Stop` (`SkeletalMeshComponent.GetAnimInstance` (`self.Mesh`)) 0.0 "/Game/ThirdPersonBP/Blueprints/GatheringMontage.GatheringMontage")
    (`self.MC_StopMontage`)
    (`/Engine/EditorBlueprintResources/StandardMacros.IsValid` (`AIBlueprintHelperLibrary.GetBlackboard` null)
      (:`Is Valid`
        (`BlackboardComponent.SetValueAsObject` (`AIBlueprintHelperLibrary.GetBlackboard` null) (`self.ResourceToGatherBBK`) (`self.CurrentResourceToGather`))
        (`BlackboardComponent.SetValueAsBool` (`AIBlueprintHelperLibrary.GetBlackboard` null) (`self.GoingToResourceBBK`) false)
        (`BlackboardComponent.SetValueAsBool` (`AIBlueprintHelperLibrary.GetBlackboard` null) (`self.ReturningToDropBBK`) false)))
    (else
      (`KismetSystemLibrary.K2_ClearTimerHandle` (`self.CollectingAnimationTH`))
      (`KismetSystemLibrary.K2_ClearTimerHandle` (`self.ActualCollectionTH`))
      (`self.FindDeposit` (`/Game/ThirdPersonBP/Blueprints/MasterDeposit.DepositType` (`self.CurrentDeposit`))))))

(fn `MoveToLocation`
  (params (InLocation :type "Vector Structure"))
  (bind _asmy_aicontroller (cast `/Game/ThirdPersonBP/Blueprints/MyAIController` (`self.GetController`)))
  (`/Game/ThirdPersonBP/Blueprints/MyAIController.MoveTo` _asmy_aicontroller InLocation))

(fn `ResourceSelected`
  (params (InResource :type "/Game/ThirdPersonBP/Blueprints/MasterResource Object Reference"))
  (set `self.CurrentResourceToGather` InResource)
  (set `self.CurrentDeposit` (`/Game/ThirdPersonBP/Blueprints/MasterResource.DepositBelongTo` (`self.CurrentResourceToGather`)))
  (`AnimInstance.Montage_Stop` (`SkeletalMeshComponent.GetAnimInstance` (`self.Mesh`)) 0.0 "/Game/ThirdPersonBP/Blueprints/GatheringMontage.GatheringMontage")
  (`self.MC_StopMontage`)
  (`/Engine/EditorBlueprintResources/StandardMacros.IsValid` (`AIBlueprintHelperLibrary.GetBlackboard` null)
    (:`Is Valid`
      (`BlackboardComponent.SetValueAsObject` (`AIBlueprintHelperLibrary.GetBlackboard` null) (`self.ResourceToGatherBBK`) (`self.CurrentResourceToGather`))
      (`BlackboardComponent.SetValueAsBool` (`AIBlueprintHelperLibrary.GetBlackboard` null) (`self.GoingToResourceBBK`) false)
      (`BlackboardComponent.SetValueAsBool` (`AIBlueprintHelperLibrary.GetBlackboard` null) (`self.ReturningToDropBBK`) false))))

(fn `StartActualCollection`
  (locals (LocalAmountToExtract :type "Float (double-precision)"))
  (bind _currentresourcetogather (`self.CurrentResourceToGather`))
  (bind _maxresourcecarry (`self.MaxResourceCarry`))
  (bind _currentresourcetogather_2 (`self.CurrentResourceToGather`))
  (bind _currentresourcetogather_3 (`self.CurrentResourceToGather`))
  (bind _returnvalue (+ (`self.CurrentResourceCarry`) (`local.LocalAmountToExtract`)))
  (bind _depositbelongto (`/Game/ThirdPersonBP/Blueprints/MasterResource.DepositBelongTo` (`self.CurrentResourceToGather`)))
  (bind _returnvalue_2 (`KismetMathLibrary.FClamp` (+ (`self.CurrentResourceCarry`) (`local.LocalAmountToExtract`)) 0.0 (`self.MaxResourceCarry`)))
  (`/Engine/EditorBlueprintResources/StandardMacros.IsValid` (`self.CurrentResourceToGather`)
    (:`Is Valid`
      (switch `/Game/ThirdPersonBP/Blueprints/ResourceEnum` (`/Game/ThirdPersonBP/Blueprints/MasterResource.ResourceType` _currentresourcetogather_3)
        (:`NewEnumerator0`
          (if (>= (- (`/Game/ThirdPersonBP/Blueprints/MasterResource.CurrentResourceCarry` _currentresourcetogather_3) (`/Game/ThirdPersonBP/Blueprints/MasterResource.ExtractionRate` _currentresourcetogather_3)) 0.0)
            (set `local.LocalAmountToExtract` (`/Game/ThirdPersonBP/Blueprints/MasterResource.ExtractionRate` _currentresourcetogather))
            (else
              (set `local.LocalAmountToExtract` (`/Game/ThirdPersonBP/Blueprints/MasterResource.CurrentResourceCarry` _currentresourcetogather))))
          (if (not (<= _returnvalue _maxresourcecarry))
            (set `local.LocalAmountToExtract` (- (`local.LocalAmountToExtract`) (- _returnvalue _maxresourcecarry))))
          (set `/Game/ThirdPersonBP/Blueprints/MasterResource.CurrentResourceCarry` (`KismetMathLibrary.FClamp` (- (`/Game/ThirdPersonBP/Blueprints/MasterResource.CurrentResourceCarry` _currentresourcetogather_2) (`local.LocalAmountToExtract`)) 0.0 (`/Game/ThirdPersonBP/Blueprints/MasterResource.MaxResourceCarry` _currentresourcetogather_2)) (`self.CurrentResourceToGather`))
          (set `self.CurrentFoodCarry` _returnvalue_2)
          (set `self.CurrentResourceCarry` _returnvalue_2)
          (set `/Game/ThirdPersonBP/Blueprints/MasterDeposit.DepositCurrentCapacity` (- (`/Game/ThirdPersonBP/Blueprints/MasterDeposit.DepositCurrentCapacity` _depositbelongto) (`local.LocalAmountToExtract`)) _depositbelongto)
          (if (== (`self.CurrentResourceCarry`) (`self.MaxResourceCarry`))
            (`AnimInstance.Montage_Stop` (`SkeletalMeshComponent.GetAnimInstance` (`self.Mesh`)) 0.0 "/Game/ThirdPersonBP/Blueprints/GatheringMontage.GatheringMontage")
            (`self.MC_StopMontage`)
            (`/Engine/EditorBlueprintResources/StandardMacros.IsValid` (`AIBlueprintHelperLibrary.GetBlackboard` null)
              (:`Is Valid`
                (`BlackboardComponent.SetValueAsBool` (`AIBlueprintHelperLibrary.GetBlackboard` null) (`self.BagFullBBK`) true)
                (`KismetSystemLibrary.K2_ClearTimerHandle` (`self.CollectingAnimationTH`))
                (`KismetSystemLibrary.K2_ClearTimerHandle` (`self.ActualCollectionTH`))
                (if (== (`/Game/ThirdPersonBP/Blueprints/MasterResource.CurrentResourceCarry` (`self.CurrentResourceToGather`)) 0.0)
                  (`KismetArrayLibrary.Array_RemoveItem` (`/Game/ThirdPersonBP/Blueprints/MasterDeposit.ResourceInDeposit` (`/Game/ThirdPersonBP/Blueprints/MasterResource.DepositBelongTo` (`self.CurrentResourceToGather`))) (`self.CurrentResourceToGather`))
                  (`self.K2_DestroyActor` (`self.CurrentResourceToGather`)))))
            (elif (== (`/Game/ThirdPersonBP/Blueprints/MasterResource.CurrentResourceCarry` (`self.CurrentResourceToGather`)) 0.0)
              (`KismetArrayLibrary.Array_RemoveItem` (`/Game/ThirdPersonBP/Blueprints/MasterDeposit.ResourceInDeposit` (`/Game/ThirdPersonBP/Blueprints/MasterResource.DepositBelongTo` (`self.CurrentResourceToGather`))) (`self.CurrentResourceToGather`))
              (`self.K2_DestroyActor` (`self.CurrentResourceToGather`))
              (`self.FindNearResourceInDeposit`))))))
    (:`Is Not Valid`
      (`AnimInstance.Montage_Stop` (`SkeletalMeshComponent.GetAnimInstance` (`self.Mesh`)) 0.0 "/Game/ThirdPersonBP/Blueprints/GatheringMontage.GatheringMontage")
      (`self.MC_StopMontage`)
      (`KismetSystemLibrary.K2_ClearTimerHandle` (`self.CollectingAnimationTH`))
      (`KismetSystemLibrary.K2_ClearTimerHandle` (`self.ActualCollectionTH`))
      (`self.FindNearResourceInDeposit`))))

(fn `StartCollectAnimation`
  (bind (_returnvalue_roll _returnvalue_pitch) (`KismetMathLibrary.BreakRotator` (`self.K2_GetActorRotation`)))
  (bind (_returnvalue_roll_2 _returnvalue_pitch_2 _returnvalue_yaw) (`KismetMathLibrary.BreakRotator` (`KismetMathLibrary.FindLookAtRotation` (`self.K2_GetActorLocation`) (`self.K2_GetActorLocation` (`self.CurrentResourceToGather`)))))
  (`/Engine/EditorBlueprintResources/StandardMacros.IsValid` (`self.CurrentResourceToGather`)
    (:`Is Valid`
      (`self.K2_SetActorRotation` (`KismetMathLibrary.MakeRotator` _returnvalue_roll _returnvalue_pitch _returnvalue_yaw))
      (bind _returnvalue (`AnimInstance.Montage_Play` (`SkeletalMeshComponent.GetAnimInstance` (`self.Mesh`)) "/Game/ThirdPersonBP/Blueprints/GatheringMontage.GatheringMontage" 1.0 "MontageLength" 0.0))
      (`self.MC_PlayMontage`)
      (bind _returnvalue_2 (`KismetSystemLibrary.K2_SetTimer` null "StartCollectAnimation" _returnvalue true))
      (set `self.CollectingAnimationTH` _returnvalue_2))
    (:`Is Not Valid`
      (`AnimInstance.Montage_Stop` (`SkeletalMeshComponent.GetAnimInstance` (`self.Mesh`)) 0.0 "/Game/ThirdPersonBP/Blueprints/GatheringMontage.GatheringMontage")
      (`self.MC_StopMontage`)
      (`KismetSystemLibrary.K2_ClearTimerHandle` (`self.CollectingAnimationTH`))
      (`KismetSystemLibrary.K2_ClearTimerHandle` (`self.ActualCollectionTH`))
      (`self.FindNearResourceInDeposit`))))

(fn `StartCollectSequence`
  (`/Engine/EditorBlueprintResources/StandardMacros.IsValid` (`self.CurrentResourceToGather`)
    (:`Is Valid`
      (if (not (`KismetSystemLibrary.K2_IsTimerActiveHandle` (`self.CollectingAnimationTH`)))
        (`|ExecutionSequence`
          (:`then_0`
            (if (not (`KismetSystemLibrary.K2_IsTimerActiveHandle` (`self.ActualCollectionTH`)))
              (bind _returnvalue (`KismetSystemLibrary.K2_SetTimer` null "StartActualCollection" 3.0 true))
              (set `self.ActualCollectionTH` _returnvalue)))
          (:`then_1`
            (`KismetSystemLibrary.K2_SetTimer` null "StartCollectAnimation" 0.01)))))
    (:`Is Not Valid`
      (`self.FindNearResourceInDeposit`))))

(fn `UserConstructionScript`)