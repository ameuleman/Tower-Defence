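; Base combat unit for a tower defense RTS that targets the nearest living actor of its enemy class and attacks it.
; EngageFight faces the target and runs a delay-based loop macro that deals Strength damage while both units can fight.
; At zero Hp it makes every actor of the attacker's class retarget, then destroys itself after a delay.
; Helper functions drive spawn, idle, attack and death states through flags on the ZombieAnimation instance.
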(event `self.ReceiveBeginPlay`
  (bind _aszombie_animation (cast `/Game/RTS_TowerDefense/Zombie/Animations/ZombieAnimation` (`SkeletalMeshComponent.GetAnimInstance` (`self.Mesh`))))
  (set `self.ZombieAnim` _aszombie_animation)
  (set `self.AttackEnded` true)
  (`self.changeTarget`)
  (`self.setSpawningAnnimation`)
  (`KismetSystemLibrary.Delay` (`self.spawnDelay`)))

(event `EventDie`
  (set `self.dying` true)
  (set `self.AttackEnded` true)
  (`self.setDyingAnnimation`)
  (`KismetSystemLibrary.Delay` (`self.deathDelay`))
  (`self.K2_DestroyActor`))

(event `EventEngageFight`
  (`self.WhileWaitTargetCheck` (and (not (or (`self.dying`) (`self.AttackEnded`) (`/Game/RTS_TowerDefense/Blueprints/fightingUnit.dying` (`self.target`)))) (`self.Attacking`)) (`self.hittingDelay`) (- (`self.hittingPeriod`) (`self.hittingDelay`))
    (:`LoopBody`
      (`self.takeDamages` (`self.target`) self))
    (:`complete`
      (`self.setIdleAnnimation`)
      (set `self.AttackEnded` true)
      (`self.changeTarget`))))

(fn `changeTarget`
  (locals (i :type Integer :default 0))
  (if (`self.AttackEnded`)
    (bind _outactors (`GameplayStatics.GetAllActorsOfClass` (`self.ennemyClass`)))
    (if (`self.changeTargetNeedInit`)
      (for _array_element _outactors
        (if (not (`/Game/RTS_TowerDefense/Blueprints/fightingUnit.dying` _array_element))
          (break)))
      (set `self.distanceToTarget` (`self.GetDistanceTo` _array_element))
      (set `self.target` _array_element))
    (for _array_element_2 _outactors
      (bind _returnvalue (`self.GetDistanceTo` _array_element_2))
      (if (and (not (`/Game/RTS_TowerDefense/Blueprints/fightingUnit.dying` _array_element_2)) (< _returnvalue (`self.distanceToTarget`)))
        (bind _output_get (set `self.target` _array_element_2))
        (set `self.distanceToTarget` _returnvalue)
        (`/Engine/EditorBlueprintResources/StandardMacros.IsValid` _output_get
          (:`Is Not Valid`
            (`self.setIdleAnnimation`)))))))

(fn `die`
  (`self.EventDie`))

(fn `engageFight`
  (if (`self.AttackEnded`)
    (set `self.AttackEnded` false)
    (set `self.Attacking` true)
    (`self.rotateToTarget`)
    (`self.setAttackingAnnimation`)
    (`self.EventEngageFight`)))

(fn `rotateToTarget`
  (bind (_returnvalue_roll _returnvalue_pitch _returnvalue_yaw) (`KismetMathLibrary.BreakRotator` (`KismetMathLibrary.FindLookAtRotation` (`self.K2_GetActorLocation`) (`self.K2_GetActorLocation` (`self.target`)))))
  (`self.K2_SetActorRotation` (`KismetMathLibrary.MakeRotator` 0.0 0.0 _returnvalue_yaw)))

(fn `setAttackingAnnimation`
  (bind _zombieanim (`self.ZombieAnim`))
  (set `/Game/RTS_TowerDefense/Zombie/Animations/ZombieAnimation.Attacking` true _zombieanim)
  (set `/Game/RTS_TowerDefense/Zombie/Animations/ZombieAnimation.Running` false _zombieanim)
  (set `/Game/RTS_TowerDefense/Zombie/Animations/ZombieAnimation.Walking` false _zombieanim))

(fn `setDyingAnnimation`
  (set `/Game/RTS_TowerDefense/Zombie/Animations/ZombieAnimation.dying` true (`self.ZombieAnim`)))

(fn `setIdleAnnimation`
  (bind _zombieanim (`self.ZombieAnim`))
  (set `/Game/RTS_TowerDefense/Zombie/Animations/ZombieAnimation.Attacking` false _zombieanim)
  (set `/Game/RTS_TowerDefense/Zombie/Animations/ZombieAnimation.Running` false _zombieanim)
  (set `/Game/RTS_TowerDefense/Zombie/Animations/ZombieAnimation.Walking` false _zombieanim))

(fn `setSpawningAnnimation`)

(fn `takeDamages`
  (params (attacker :type "/Game/RTS_TowerDefense/Blueprints/fightingUnit Object Reference"))
  (bind _output_get (set `self.hp` (- (`self.hp`) (`/Game/RTS_TowerDefense/Blueprints/fightingUnit.strength` attacker))))
  (if (<= _output_get 0)
    (set `self.dying` true)
    (bind _outactors (`GameplayStatics.GetAllActorsOfClass` (`GameplayStatics.GetObjectClass` attacker)))
    (for _array_element _outactors
      (set `/Game/RTS_TowerDefense/Blueprints/fightingUnit.Attacking` false _array_element)
      (`self.changeTarget` _array_element))
    (`self.die`)))

(fn `UserConstructionScript`)